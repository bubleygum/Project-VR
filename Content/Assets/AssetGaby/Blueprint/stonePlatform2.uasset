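; Stone platform actor that detects whether a WolfStatue rests within its Box volume, likely as part of a statue placement puzzle.
; Every Tick it queries the Box's overlapping actors filtered to WolfStatue instead of using overlap events.
; The result sets the Wolf flag and switches the static mesh between the Glow1 material and the default platform material.
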(event `self.ReceiveTick`
  (params (DeltaSeconds :type "Float (single-precision)"))
  (if (!= (`KismetArrayLibrary.Array_Length` (`PrimitiveComponent.GetOverlappingActors` (`self.Box`) "/Game/Assets/AssetGaby/Blueprint/wolfStatue.wolfStatue_C")) 0)
    (set `self.wolf` true)
    (`PrimitiveComponent.SetMaterial` (`self.StaticMesh`) 0 "/Game/Assets/AssetGaby/Meshes/sculptjanuary2021-day-05-magic-gate/source/Day_05_-_Magic_Gate_optim1/glow1.glow1")
    (else
      (set `self.wolf` false)
      (`PrimitiveComponent.SetMaterial` (`self.StaticMesh`) 0 "/Game/Assets/AssetGaby/Meshes/stone-platform/source/platformMaterial.platformMaterial"))))

(fn `UserConstructionScript`)