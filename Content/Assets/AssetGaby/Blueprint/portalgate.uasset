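; Portal gate actor that spins two magic gate rings and sends the player to the "Mika" level on contact.
; Tick calls Play on the Rotate timeline, whose track yaws the rings in opposite directions.
; Each timeline update also polls the Box for overlap with the player character, printing a debug message and opening the level, rather than using an overlap event.
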(event `self.ReceiveTick`
  (params (DeltaSeconds :type "Float (single-precision)"))
  (bind (_direction _rotate) (`Timeline|rotate`)
    (:`Update`
      (`SceneComponent.K2_SetRelativeRotation` (`self.Day_05_-_Magic_Gate_optim2_ring_001`) (`KismetMathLibrary.MakeRotator` 0.0 0.0 _rotate) false false)
      (`SceneComponent.K2_SetRelativeRotation` (`self.Day_05_-_Magic_Gate_optim2_ring_002`) (`KismetMathLibrary.MakeRotator` 0.0 0.0 (* _rotate -1.0)) false false)
      (if (`PrimitiveComponent.IsOverlappingActor` (`self.Box`) (`GameplayStatics.GetPlayerCharacter` 0))
        (`KismetSystemLibrary.PrintString` "Hello")
        (`GameplayStatics.OpenLevel` " Mika")))))

(fn `UserConstructionScript`)