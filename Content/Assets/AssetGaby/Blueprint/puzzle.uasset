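; Stone puzzle actor that moves a portal once three stones report their animal flags.
; Tick checks the Leopard, Lion and Wolf flags in sequence on StonePlatform, Stone1 and Stone2.
; When all three are true, a timeline drives the Portal's relative X location.
; If only Wolf is false, a second timeline sets this actor's own relative X to its negated track value.
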(event `self.ReceiveBeginPlay`)

(event `self.ReceiveTick`
  (params (DeltaSeconds :type "Float (single-precision)"))
  (if (`/Game/Assets/AssetGaby/Blueprint/stonePlatform.leopard` (`self.stonePlatform`))
    (if (`/Game/Assets/AssetGaby/Blueprint/stonePlatform1.lion` (`self.stone1`))
      (if (`/Game/Assets/AssetGaby/Blueprint/stonePlatform2.wolf` (`self.stone2`))
        (bind (_direction _newtrack_0) (`Timeline|Timeline`)
          (:`Update`
            (`self.K2_SetActorRelativeLocation` (`self.portal`) (`KismetMathLibrary.MakeVector` _newtrack_0) false false)))
        (else
          (bind (_direction_2 _newtrack_0_2) (`Timeline|Timeline_0`)
            (:`Update`
              (`self.K2_SetActorRelativeLocation` (`KismetMathLibrary.MakeVector` (* _newtrack_0_2 -1.0))))))))))

(fn `UserConstructionScript`)